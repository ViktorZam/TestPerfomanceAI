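; BP_PawnCamera is a free-moving camera pawn with mouse-cursor input, driven by Enhanced Input.
; WASD moves it along the camera's yaw, or along its full rotation with interpolation while right mouse is held.
; Holding right mouse also rotates the camera, hiding the cursor and pinning it in place; pressing it first calls CallMove.
; Left mouse sets the HUD's start mouse position, and G prints the BP_TopDownCharacter count.
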(event Input|EnhancedActionEvents|EnhancedInputActionIA_LeftMouse
  (params (ActionValue :type Boolean) (ElapsedSeconds :type Float%20%28double-precision%29) (TriggeredSeconds :type Float%20%28double-precision%29) (InputAction :type Input%20Action%20Object%20Reference :default "/Game/Input/Actions/IA_LeftMouse.IA_LeftMouse"))
  (:Started
    (Variables|Default|SetLeftMouseHolding? true)
    (Default|SetStartMousePosition (Variables|Default|GetHUD)))
  (:Completed
    (Variables|Default|SetLeftMouseHolding? false)))

(event Input|EnhancedActionEvents|EnhancedInputActionIA_MoveCameraWS
  (params (ActionValue :type Float%20%28double-precision%29) (ElapsedSeconds :type Float%20%28double-precision%29) (TriggeredSeconds :type Float%20%28double-precision%29) (InputAction :type Input%20Action%20Object%20Reference :default "/Game/Input/Actions/IA_MoveCameraWS.IA_MoveCameraWS"))
  (bind _returnvalue (Transformation|GetActorLocation))
  (:Triggered
    (if (Variables|Default|GetRightMouseHolding?)
      (Transformation|SetActorLocation (Math|Interpolation|VInterpTo _returnvalue (+ _returnvalue (* (Math|Vector|GetForwardVector (Variables|/Script/Engine.SceneComponent|GetRelativeRotation (Variables|Default|GetCamera))) ActionValue 1e+01)) (Utilities|Time|GetWorldDeltaSeconds) 6e+01) true false)
      (else
        (Transformation|AddActorWorldOffset (* ActionValue (Math|Vector|GetForwardVector (Math|Rotator|MakeRotator 0.0 0.0 (.yaw (Variables|/Script/Engine.SceneComponent|GetRelativeRotation (Variables|Default|GetCamera))))) 1e+01) true)))))

(event Input|EnhancedActionEvents|EnhancedInputActionIA_MoveCameraAD
  (params (ActionValue :type Float%20%28double-precision%29) (ElapsedSeconds :type Float%20%28double-precision%29) (TriggeredSeconds :type Float%20%28double-precision%29) (InputAction :type Input%20Action%20Object%20Reference :default "/Game/Input/Actions/IA_MoveCameraAD.IA_MoveCameraAD"))
  (bind _returnvalue (Transformation|GetActorLocation))
  (:Triggered
    (if (Variables|Default|GetRightMouseHolding?)
      (Transformation|SetActorLocation (Math|Interpolation|VInterpTo _returnvalue (+ _returnvalue (* (Math|Vector|GetRightVector (Variables|/Script/Engine.SceneComponent|GetRelativeRotation (Variables|Default|GetCamera))) ActionValue 1e+01)) (Utilities|Time|GetWorldDeltaSeconds) 6e+01) true false)
      (else
        (Transformation|AddActorWorldOffset (* ActionValue (Math|Vector|GetRightVector (Math|Rotator|MakeRotator 0.0 0.0 (.yaw (Variables|/Script/Engine.SceneComponent|GetRelativeRotation (Variables|Default|GetCamera))))) 1e+01) true)))))

(event Input|EnhancedActionEvents|EnhancedInputActionIA_RotateCamera
  (params (ActionValue :type Vector%202D%20Structure) (ElapsedSeconds :type Float%20%28double-precision%29) (TriggeredSeconds :type Float%20%28double-precision%29) (InputAction :type Input%20Action%20Object%20Reference :default "/Game/Input/Actions/IA_RotateCamera.IA_RotateCamera"))
  (bind (_x _y) (Math|Vector2D|BreakVector2D ActionValue))
  (bind _returnvalue (Utilities|Time|GetWorldDeltaSeconds))
  (bind _camera (Variables|Default|GetCamera))
  (bind _lastmouseposition (Variables|Default|GetLastMousePosition))
  (bind _camera_2 (Variables|Default|GetCamera))
  (bind _returnvalue_2 (* _y 2.0))
  (bind _returnvalue_3 (* _x 2.0))
  (bind _relativerotation (Variables|/Script/Engine.SceneComponent|GetRelativeRotation _camera_2))
  (bind _relativerotation_2 (Variables|/Script/Engine.SceneComponent|GetRelativeRotation _camera))
  (bind _returnvalue_4 (+ (.pitch _relativerotation) _returnvalue_2))
  (bind _returnvalue_5 (+ (.yaw _relativerotation) _returnvalue_3))
  (bind _returnvalue_6 (Math|Interpolation|RInterpTo _relativerotation_2 (Math|Rotator|MakeRotator 0.0 _returnvalue_4 _returnvalue_5) _returnvalue 1e+02))
  (:Triggered
    (if (Variables|Default|GetRightMouseHolding?)
      (Class|PlayerController|SetMouseLocation (Game|GetPlayerController 0) (Math|Float|Truncate (.x _lastmouseposition)) (Math|Float|Truncate (.y _lastmouseposition)))
      (Transformation|SetRelativeRotation (Variables|Default|GetCamera) (Math|Rotator|MakeRotator 0.0 (.pitch _returnvalue_6) (.yaw _returnvalue_6)) false false))))

(event Input|EnhancedActionEvents|EnhancedInputActionIA_RightMouse
  (params (ActionValue :type Boolean) (ElapsedSeconds :type Float%20%28double-precision%29) (TriggeredSeconds :type Float%20%28double-precision%29) (InputAction :type Input%20Action%20Object%20Reference :default "/Game/Input/Actions/IA_RightMouse.IA_RightMouse"))
  (bind _returnvalue (Game|GetPlayerController 0))
  (bind (_locationx _locationy) (Game|Player|GetMousePosition _returnvalue))
  (:Triggered
    (Variables|/Script/Engine.PlayerController|SetbShowMouseCursor (Game|GetPlayerController 0) false))
  (:Started
    (Default|CallMove)
    (Variables|Default|SetRightMouseHolding? true)
    (Variables|Default|SetLastMousePosition (Math|Vector2D|MakeVector2D _locationx _locationy)))
  (:Completed
    (Variables|Default|SetRightMouseHolding? false)
    (Variables|/Script/Engine.PlayerController|SetbShowMouseCursor (Game|GetPlayerController 0) true)))

(event EventBeginPlay
  (bind _returnvalue (Game|GetPlayerController 0))
  (bind _returnvalue_2 (PlayerController|LocalPlayerSubsystems|GetEnhancedInputLocalPlayerSubsystem _returnvalue))
  (Utilities|IsValid _returnvalue_2
    (:Is%20Valid
      (Input|AddMappingContext _returnvalue_2 "/Game/Input/IMC_Default.IMC_Default" 0 "(bIgnoreAllPressedKeysUntilRelease=True,bForceImmediately=False)")
      (Input|SetInputModeGameandUI (Game|GetPlayerController 0) 0 "DoNotLock" false false)
      (bind _asbp_hud (Utilities|Casting|CastToBP_HUD (HUD|GetHUD (Game|GetPlayerController 0))))
      (Variables|Default|SetHUD _asbp_hud))))

(event Input|KeyboardEvents|G
  (params (Key :type Key%20Structure :default "None"))
  (:Pressed
    (bind _outactors (Actor|GetAllActorsOfClass "/Game/Blueprints/BP_TopDownCharacter.BP_TopDownCharacter_C"))
    (Development|PrintString (Utilities|String|ToString(Integer) (Utilities|Array|Length _outactors)))))

(fn ConstructionScript)

(fn GetCameraPawn
  (return self))